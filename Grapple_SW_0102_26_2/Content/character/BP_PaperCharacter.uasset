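; Player character that moves along world X under a level cine camera and can climb surfaces.
; IA_Climb toggles climbing, using a forward trace to latch the capsule to a wall, with Flying mode as the climb state.
; IA_PaperMove then drives movement along the actor's right and up vectors, while a timeline keeps it facing the wall.
; Stepped downward traces find the ledge top, and another timeline lerps the character onto it.
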(event Custom|climb%20movement
  (params (WorldDirection :type Vector) (ScaleValue :type Float%20%28single-precision%29))
  ;[0.15 0.15 0.15 0.5] the start climbing logic
  (bind (_hit _success) (CallFunction|LatchOntoSurface 1.2e+02))
  ;;[0.15 0.15 0.15 0.5] is there a platform?
  (if _success
    ;;[0.15 0.15 0.15 0.5] allowing the player to climb up and down
    (Pawn|Input|AddMovementInput WorldDirection ScaleValue false)
    (CallFunction|LedgePosition)
    ;;[0.15 0.15 0.15 0.5] making the snapping more smooth with a timeline
    (bind _rotation (Timeline|climbing%20alignment PlayFromStart)
      (:Update
        ;;[0.15 0.15 0.15 0.5] snaps the player rotation to ensure they always face the platform
        (Transformation|SetActorRotation (Math|Rotator|Lerp(Rotator) (Transformation|GetActorRotation) (Math|Rotator|MakeRotfromX (* (.Normal (Collision|BreakHitResult _hit)) -1.0)) _rotation))))))

(event Custom|stop%20climbing
  (bind _charactermovement (Variables|Character|GetCharacterMovement))
  ;[0.15 0.15 0.15 0.5] changing the movement to falling
  ;;[0.15 0.15 0.15 0.5] it's falling not walking as we don't know the player height at time of falling
  (Pawn|Components|CharacterMovement|SetMovementMode _charactermovement "MOVE_Falling" 0)
  ;;[0.15 0.15 0.15 0.5] set player back to rotating the correct direction
  (Variables|/Script/Engine.CharacterMovementComponent|SetbOrientRotationToMovement _charactermovement true)
  ;;[0.15 0.15 0.15 0.5] rotation back to being player controlled
  (Utilities|FlowControl|Delay 0.5)
  (Transformation|SetActorRotation (Math|Rotator|MakeRotator 0.0 0.0 (.yaw (Transformation|GetActorRotation)))))

(event Custom|ledge%20position
  (bind _returnvalue (Transformation|GetActorLocation))
  (bind _returnvalue_2 (Transformation|GetActorRotation))
  (bind _returnvalue_3 (+ _returnvalue "0.000000,0.000000,100.000000"))
  ;[0.15 0.15 0.15 0.5] where is the ledge of the wall?
  ;;[0.15 0.15 0.15 0.5] detecting the wall
  (bind (_outhit _returnvalue_4) (Collision|LineTraceByChannel _returnvalue_3 (+ _returnvalue_3 (* (Math|Vector|GetForwardVector (Transformation|GetActorRotation)) 1e+02)) "TraceTypeQuery1" false 0 "None"))
  ;;[0.15 0.15 0.15 0.5] detecting the end of the wall [ledge]
  (if (not _returnvalue_4)
    (bind _index (Utilities|FlowControl|ForLoopwithBreak 0 20 :!label _label)
      (:LoopBody
        ;;[0.15 0.15 0.15 0.5] detecting end of wall
        (bind (_outhit_2 _returnvalue_5) (Collision|LineTraceByChannel (+ (* (* _index 3) (Math|Vector|GetForwardVector (Transformation|GetActorRotation))) (+ (.TraceStart (Collision|BreakHitResult _outhit)) "0.000000,0.000000,90.000000")) (- (+ (* (* _index 3) (Math|Vector|GetForwardVector (Transformation|GetActorRotation))) (+ (.TraceStart (Collision|BreakHitResult _outhit)) "0.000000,0.000000,90.000000")) "0.000000,0.000000,100.000000") "TraceTypeQuery1" false 0 "None"))
        ;;[0.15 0.15 0.15 0.5] break loop after then 0
        (if _returnvalue_5
          (Utilities|FlowControl|Sequence
            (:then_0
              ;;[0.15 0.15 0.15 0.5] dont repeat
              (Utilities|FlowControl|DoOnce false
                (:Completed
                  ;;[0.15 0.15 0.15 0.5] making the movement smooth
                  (bind _newtrack_0 (Timeline|Timeline PlayFromStart)
                    (:Update
                      ;;[0.15 0.15 0.15 0.5] chnaging to new location and set player movement to fall due to player height
                      (Transformation|SetActorLocation (Math|Vector|Lerp(Vector) (Transformation|GetActorLocation) (+ (.Location (Collision|BreakHitResult _outhit_2)) (+ (Math|Vector|GetForwardVector _returnvalue_2) 12.0) (+ (Math|Vector|GetUpVector _returnvalue_2) 7.0)) _newtrack_0) false false))))))
            (:then_1
              (goto _label Break))))))))

(event Input|EnhancedActionEvents|EnhancedInputActionIA_PaperMove
  (params (ActionValue :type Float%20%28double-precision%29) (ElapsedSeconds :type Float%20%28double-precision%29) (TriggeredSeconds :type Float%20%28double-precision%29) (InputAction :type Input%20Action%20Object%20Reference :default "/Game/character/Inputs/IA_PaperMove.IA_PaperMove"))
  ;[0.15 0.15 0.15 0.5] creating the player input
  ;;[0.15 0.15 0.15 0.5] are we walking or climbing?
  (switch Utilities|FlowControl|Switch|SwitchonEMovementMode (Variables|/Script/Engine.CharacterMovementComponent|GetMovementMode (Variables|Character|GetCharacterMovement))
    (:MOVE_Walking
      ;;[0.15 0.15 0.15 0.5] movement logic and locking the world direction
      (Pawn|Input|AddMovementInput "1.000000,0.000000,0.000000" ActionValue false :!label _label))
    (:MOVE_Falling
      (goto _label))
    (:MOVE_Flying
      ;;[0.15 0.15 0.15 0.5] adding the left ad right movement to climbing
      (CallFunction|ClimbMovement (Transformation|GetActorRightVector) ActionValue)
      ;;[0.15 0.15 0.15 0.5] adding the up and down movement to climbig
      (CallFunction|ClimbMovement (Transformation|GetActorUpVector) ActionValue))))

(event Input|EnhancedActionEvents|EnhancedInputActionIA_Climb
  (params (ActionValue :type Boolean) (ElapsedSeconds :type Float%20%28double-precision%29) (TriggeredSeconds :type Float%20%28double-precision%29) (InputAction :type Input%20Action%20Object%20Reference :default "/Game/character/Inputs/IA_Climb.IA_Climb"))
  (bind _charactermovement (Variables|Character|GetCharacterMovement))
  (bind _capsulecomponent (Variables|Default|GetCapsuleComponent))
  ;[0.15 0.15 0.15 0.5] creating input to climb
  (:Started
    ;;[0.15 0.15 0.15 0.5] is there a platform yes or no?
    (if (Utilities|Enum|NotEqual(Enum) (Variables|/Script/Engine.CharacterMovementComponent|GetMovementMode (Variables|Character|GetCharacterMovement)) "MOVE_Flying")
      ;;[0.15 0.15 0.15 0.5] latch to surface if within certain distance.
      (bind (_hit _success) (CallFunction|LatchOntoSurface 1e+02))
      ;;[0.15 0.15 0.15 0.5] is there a platform to latch onto?
      (if _success
        ;;[0.15 0.15 0.15 0.5] changing movement to climbing
        (Pawn|Components|CharacterMovement|SetMovementMode _charactermovement "MOVE_Flying" 0)
        ;;[0.15 0.15 0.15 0.5] keeps the player facing the wall
        (Variables|/Script/Engine.CharacterMovementComponent|SetbOrientRotationToMovement _charactermovement false)
        ;;[0.15 0.15 0.15 0.5] setting the latching location
        (Components|MoveComponentTo _capsulecomponent (+ (.Location (Collision|BreakHitResult _hit)) (* (Variables|/Script/Engine.CapsuleComponent|GetCapsuleRadius _capsulecomponent) (.Normal (Collision|BreakHitResult _hit)))) (Math|Rotator|MakeRotfromX (* (.Normal (Collision|BreakHitResult _hit)) -1.0)) false false 0.2 false))
      (else
        ;;[0.15 0.15 0.15 0.5] stop climbing if no platform
        (CallFunction|StopClimbing)))))

(event EventBeginPlay
  (bind _returnvalue (Game|GetPlayerController 0))
  ;[0.15 0.15 0.15 0.5] adding maping context to use input actions to move
  (bind _returnvalue_2 (Actor|GetActorOfClass "/Script/Engine.CameraActor"))
  (bind _ascine_camera_actor (Utilities|Casting|CastToCineCameraActor _returnvalue_2))
  (Game|Player|SetViewTargetwithBlend _returnvalue _ascine_camera_actor 0.0 "VTBlend_Linear" 0.0 false)
  (Input|AddMappingContext (PlayerController|LocalPlayerSubsystems|GetEnhancedInputLocalPlayerSubsystem _returnvalue) "/Game/character/Inputs/IMC_PaperPlayer.IMC_PaperPlayer" 0 "(bIgnoreAllPressedKeysUntilRelease=True,bForceImmediately=False,bNotifyUserSettings=False)"))

(event Collision|EventActorBeginOverlap
  (params (OtherActor :type Actor%20Object%20Reference)))

(event EventTick
  (params (DeltaSeconds :type Float%20%28single-precision%29)))

(fn ConstructionScript)

(fn LatchOntoSurface
  (params (attach%20distance :type Float%20%28double-precision%29))
  (bind _returnvalue (Transformation|GetActorLocation))
  ;[0.15 0.15 0.15 0.5] attaching to platform function
  ;;[0.15 0.15 0.15 0.5] line trace to detect platform
  (bind (_outhit _returnvalue_2) (Collision|LineTraceByChannel _returnvalue (+ _returnvalue (* (Math|Vector|GetForwardVector (Transformation|GetActorRotation)) attach%20distance)) "TraceTypeQuery1" false 0 "None"))
  ;;[0.15 0.15 0.15 0.5] return node to check if there is a platformand feed this back to the player
  (return _outhit _returnvalue_2))